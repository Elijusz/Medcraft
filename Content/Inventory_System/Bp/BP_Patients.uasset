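; Patient station actor that registers itself on the side-scroller character on sphere overlap and manages the pool of operable patients.
; It opens and closes patient and operation widgets, guarded by resettable DoOnce nodes, updating character flags and refreshing the inventory.
; AddPatients moves entries from AddablePatients into Patients at player levels two to four.
; Both arrays and the level persist through a SavePatients save slot.
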(event OnComponentBeginOverlap(Sphere)
  (params (OverlappedComponent :type Primitive%20Component%20Object%20Reference) (OtherActor :type Actor%20Object%20Reference) (OtherComp :type Primitive%20Component%20Object%20Reference) (OtherBodyIndex :type Integer) (bFromSweep :type Boolean) (SweepResult :type Hit%20Result%20Structure%20%28by%20ref%29))
  (bind _as2dside_scroller_character (Utilities|Casting|CastTo2DSideScrollerCharacter OtherActor))
  (Variables|/Game/2DSideScrollerBP/Blueprints/2DSideScrollerCharacter.2DSideScrollerCharacter_C|SetPatients _as2dside_scroller_character self))

(event Custom|ShowOperationWidget
  (params (2DsideScroll :type 2D%20Side%20Scroller%20Character%20Object%20Reference))
  (bind _patient (Variables|Default|GetPatient))
  (Utilities|FlowControl|DoOnce false
    (:Completed
      (bind _output_get (Variables|Default|Set2DSideScroller 2DsideScroll))
      (bind _returnvalue (UserInterface|CreateWidget "/Game/Inventory_System/Widgets/OperationWidget.OperationWidget_C" 0 self (.Time (Utilities|Struct|BreakS_Patient_Info (Utilities|GetClassDefaults _patient))) _patient (Variables|/Game/2DSideScrollerBP/Blueprints/2DSideScrollerCharacter.2DSideScrollerCharacter_C|GetInventoryRef _output_get) 0))
      (Variables|Default|SetOperationWidget _returnvalue)
      (Default|InIt (Variables|Default|GetOperationWidget) _patient)
      (Class|UserWidget|SetPositioninViewport (Variables|Default|GetOperationWidget) "(X=0.000000,Y=0.000000)" false)
      (Class|UserWidget|SetAnchorsinViewport (Variables|Default|GetOperationWidget) (Utilities|Struct|MakeAnchors "(X=0.500000,Y=0.200000)" "(X=0.500000,Y=0.200000)"))
      (Class|UserWidget|SetAlignmentinViewport (Variables|Default|GetOperationWidget) "(X=0.500000,Y=0.200000)")
      (UserInterface|Viewport|AddtoViewport (Variables|Default|GetOperationWidget) 6)
      (Default|HideInventory (Variables|/Game/2DSideScrollerBP/Blueprints/2DSideScrollerCharacter.2DSideScrollerCharacter_C|GetInventoryRef (Variables|Default|Get2DSideScroller)))
      (Default|ShowInventory (Variables|/Game/2DSideScrollerBP/Blueprints/2DSideScrollerCharacter.2DSideScrollerCharacter_C|GetInventoryRef (Variables|Default|Get2DSideScroller)))
      (Variables|/Game/2DSideScrollerBP/Blueprints/2DSideScrollerCharacter.2DSideScrollerCharacter_C|SetIsOperationOpen? (Variables|Default|Get2DSideScroller) true))))

(event Custom|HideOperationWidget
  (bind _patient (Variables|Default|GetPatient))
  (Variables|/Game/2DSideScrollerBP/Blueprints/2DSideScrollerCharacter.2DSideScrollerCharacter_C|SetIsOperationOpen? (Variables|Default|Get2DSideScroller) false)
  (if (Variables|/Game/Inventory_System/Bp/BP_Inventory.BP_Inventory_C|GetIsVisable? (Variables|/Game/2DSideScrollerBP/Blueprints/2DSideScrollerCharacter.2DSideScrollerCharacter_C|GetInventoryRef (Variables|Default|Get2DSideScroller)))
    (Default|HideInventory (Variables|/Game/2DSideScrollerBP/Blueprints/2DSideScrollerCharacter.2DSideScrollerCharacter_C|GetInventoryRef (Variables|Default|Get2DSideScroller)))
    (Default|ShowInventory (Variables|/Game/2DSideScrollerBP/Blueprints/2DSideScrollerCharacter.2DSideScrollerCharacter_C|GetInventoryRef (Variables|Default|Get2DSideScroller))))
  (Widget|RemovefromParent (Variables|Default|GetOperationWidget))
  (Variables|Default|SetPatientsWidget 0)
  (Utilities|FlowControl|DoOnce false) ; enters at Reset
)

(event Custom|OnPatientsOpen
  (params (2DsideScroll :type 2D%20Side%20Scroller%20Character%20Object%20Reference))
  (Utilities|FlowControl|DoOnce false
    (:Completed
      (Variables|Default|Set2DSideScroller 2DsideScroll)
      (bind _returnvalue (UserInterface|CreateWidget "/Game/Inventory_System/Widgets/PatientsWidget.PatientsWidget_C" 0 self (Variables|Default|Get2DSideScroller)))
      (Variables|Default|SetPatientsWidget _returnvalue)
      (Class|UserWidget|SetPositioninViewport :self (Variables|Default|GetPatientsWidget) :bRemoveDPIScale false)
      (Class|UserWidget|SetAnchorsinViewport (Variables|Default|GetPatientsWidget) (Utilities|Struct|MakeAnchors "(X=1.000000,Y=1.000000)" "(X=1.000000,Y=1.000000)"))
      (Class|UserWidget|SetAlignmentinViewport (Variables|Default|GetPatientsWidget) "(X=1.000000,Y=1.000000)")
      (UserInterface|Viewport|AddtoViewport (Variables|Default|GetPatientsWidget) 6)
      (Default|HideInventory (Variables|/Game/2DSideScrollerBP/Blueprints/2DSideScrollerCharacter.2DSideScrollerCharacter_C|GetInventoryRef (Variables|Default|Get2DSideScroller)))
      (Default|ShowInventory (Variables|/Game/2DSideScrollerBP/Blueprints/2DSideScrollerCharacter.2DSideScrollerCharacter_C|GetInventoryRef (Variables|Default|Get2DSideScroller)))
      (Variables|/Game/2DSideScrollerBP/Blueprints/2DSideScrollerCharacter.2DSideScrollerCharacter_C|SetIsPatientsOpen? (Variables|Default|Get2DSideScroller) true))))

(event Custom|OnPatientsExit
  (Variables|/Game/2DSideScrollerBP/Blueprints/2DSideScrollerCharacter.2DSideScrollerCharacter_C|SetIsPatientsOpen? (Variables|Default|Get2DSideScroller) false)
  (if (Variables|/Game/Inventory_System/Bp/BP_Inventory.BP_Inventory_C|GetIsVisable? (Variables|/Game/2DSideScrollerBP/Blueprints/2DSideScrollerCharacter.2DSideScrollerCharacter_C|GetInventoryRef (Variables|Default|Get2DSideScroller)))
    (Default|HideInventory (Variables|/Game/2DSideScrollerBP/Blueprints/2DSideScrollerCharacter.2DSideScrollerCharacter_C|GetInventoryRef (Variables|Default|Get2DSideScroller)))
    (Default|ShowInventory (Variables|/Game/2DSideScrollerBP/Blueprints/2DSideScrollerCharacter.2DSideScrollerCharacter_C|GetInventoryRef (Variables|Default|Get2DSideScroller))))
  (Widget|RemovefromParent (Variables|Default|GetPatientsWidget))
  (Variables|Default|SetPatientsWidget 0)
  (Utilities|FlowControl|DoOnce false) ; enters at Reset
)

(event Collision|EventActorBeginOverlap
  (params (OtherActor :type Actor%20Object%20Reference)))

(fn ConstructionScript)

(fn GetOperatedPatient
  (params (OperatedPatient :type 0BP%20Master%20Patient%20Class%20Reference))
  (Variables|Default|SetPatient OperatedPatient)
  (return))

(fn RemovefromArray
  (params (RemovePatient :type 0BP%20Master%20Patient%20Class%20Reference))
  (Utilities|Array|RemoveItem (Variables|Default|GetPatients) RemovePatient)
  (return))

(fn LoadPatients
  (Utilities|IsValid (Variables|Default|GetSaveGameObject)
    (:Is%20Valid
      _)
    (:Is%20Not%20Valid
      (bind _returnvalue (SaveGame|LoadGamefromSlot "PatientsSave"))
      (bind _assave_patients (Utilities|Casting|CastToSavePatients _returnvalue)
        (:then
          (Variables|Default|SetSaveGameObject _assave_patients))
        (:CastFailed
          (return)))))
  (Variables|Default|SetPatients (Variables|/Game/Inventory_System/Bp/SaveGame/SavePatients.SavePatients_C|GetSavedPatients (Variables|Default|GetSaveGameObject)))
  (Variables|Default|SetAddablePatients (Variables|/Game/Inventory_System/Bp/SaveGame/SavePatients.SavePatients_C|GetSavedAddablePatients (Variables|Default|GetSaveGameObject)))
  (Variables|Default|SetLevel (Variables|/Game/Inventory_System/Bp/SaveGame/SavePatients.SavePatients_C|GetSavedPatientLevel (Variables|Default|GetSaveGameObject)))
  (return))

(fn SavePatients
  (Utilities|IsValid (Variables|Default|GetSaveGameObject)
    (:Is%20Valid
      _)
    (:Is%20Not%20Valid
      (bind _returnvalue (SaveGame|CreateSaveGameObject "/Game/Inventory_System/Bp/SaveGame/SavePatients.SavePatients_C"))
      (bind _assave_patients (Utilities|Casting|CastToSavePatients _returnvalue)
        (:then
          (Variables|Default|SetSaveGameObject _assave_patients))
        (:CastFailed
          (return)))))
  (Variables|/Game/Inventory_System/Bp/SaveGame/SavePatients.SavePatients_C|SetSavedPatients (Variables|Default|GetSaveGameObject) (Variables|Default|GetPatients))
  (Variables|/Game/Inventory_System/Bp/SaveGame/SavePatients.SavePatients_C|SetSavedAddablePatients (Variables|Default|GetSaveGameObject) (Variables|Default|GetAddablePatients))
  (Variables|/Game/Inventory_System/Bp/SaveGame/SavePatients.SavePatients_C|SetSavedPatientLevel (Variables|Default|GetSaveGameObject) (Variables|Default|GetLevel))
  (SaveGame|SaveGametoSlot (Variables|Default|GetSaveGameObject) "PatientsSave")
  (return))

(fn AddPatients
  (bind _addablepatients (Variables|Default|GetAddablePatients))
  (bind _addablepatients_2 (Variables|Default|GetAddablePatients))
  (bind _addablepatients_3 (Variables|Default|GetAddablePatients))
  (bind _addablepatients_4 (Variables|Default|GetAddablePatients))
  (bind _addablepatients_5 (Variables|Default|GetAddablePatients))
  (bind _addablepatients_6 (Variables|Default|GetAddablePatients))
  (bind _addablepatients_7 (Variables|Default|GetAddablePatients))
  (bind _addablepatients_8 (Variables|Default|GetAddablePatients))
  (bind _addablepatients_9 (Variables|Default|GetAddablePatients))
  (bind _output (Utilities|Array|Get(acopy) _addablepatients))
  (bind _output_2 (Utilities|Array|Get(acopy) _addablepatients_9))
  (bind _output_3 (Utilities|Array|Get(acopy) _addablepatients_2))
  (bind _output_4 (Utilities|Array|Get(acopy) _addablepatients_3))
  (bind _output_5 (Utilities|Array|Get(acopy) _addablepatients_4))
  (bind _output_6 (Utilities|Array|Get(acopy) _addablepatients_5))
  (bind _output_7 (Utilities|Array|Get(acopy) _addablepatients_6))
  (bind _output_8 (Utilities|Array|Get(acopy) _addablepatients_7))
  (bind _output_9 (Utilities|Array|Get(acopy) _addablepatients_8))
  (bind _as2dside_scroller_character (Utilities|Casting|CastTo2DSideScrollerCharacter (Game|GetPlayerCharacter 0)))
  (if (== (Variables|/Game/Inventory_System/Bp/LevelingSystem/LevelingSystem.LevelingSystem_C|GetCurrentLevel (Variables|/Game/2DSideScrollerBP/Blueprints/2DSideScrollerCharacter.2DSideScrollerCharacter_C|GetLevelingSystem _as2dside_scroller_character)) 2)
    (Utilities|Array|Add (Variables|Default|GetPatients) _output_7)
    (Utilities|Array|RemoveItem (Variables|Default|GetAddablePatients) _output_7)
    (Utilities|Array|Add (Variables|Default|GetPatients) _output_9)
    (Utilities|Array|RemoveItem (Variables|Default|GetAddablePatients) _output_9)
    (Utilities|Array|Add (Variables|Default|GetPatients) _output_8)
    (Utilities|Array|RemoveItem (Variables|Default|GetAddablePatients) _output_8)
    (elif (== (Variables|/Game/Inventory_System/Bp/LevelingSystem/LevelingSystem.LevelingSystem_C|GetCurrentLevel (Variables|/Game/2DSideScrollerBP/Blueprints/2DSideScrollerCharacter.2DSideScrollerCharacter_C|GetLevelingSystem _as2dside_scroller_character)) 3)
      (Utilities|Array|Add (Variables|Default|GetPatients) _output_5)
      (Utilities|Array|RemoveItem (Variables|Default|GetAddablePatients) _output_5)
      (Utilities|Array|Add (Variables|Default|GetPatients) _output_6)
      (Utilities|Array|RemoveItem (Variables|Default|GetAddablePatients) _output_6)
      (Utilities|Array|Add (Variables|Default|GetPatients) _output_2)
      (Utilities|Array|RemoveItem (Variables|Default|GetAddablePatients) _output_2)
      (Utilities|Array|Add (Variables|Default|GetPatients) _output)
      (Utilities|Array|RemoveItem (Variables|Default|GetAddablePatients) _output)
      (elif (== (Variables|/Game/Inventory_System/Bp/LevelingSystem/LevelingSystem.LevelingSystem_C|GetCurrentLevel (Variables|/Game/2DSideScrollerBP/Blueprints/2DSideScrollerCharacter.2DSideScrollerCharacter_C|GetLevelingSystem _as2dside_scroller_character)) 4)
        (Utilities|Array|Add (Variables|Default|GetPatients) _output_3)
        (Utilities|Array|RemoveItem (Variables|Default|GetAddablePatients) _output_3)
        (Utilities|Array|Add (Variables|Default|GetPatients) _output_4)
        (Utilities|Array|RemoveItem (Variables|Default|GetAddablePatients) _output_4)))))