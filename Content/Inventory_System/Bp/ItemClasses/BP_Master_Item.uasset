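; BP_Master_Item is the master item Blueprint for the inventory system, defining what happens when an item is used.
; On EventOnUsed, it checks the CanBeUsed flag in ItemInfo and prints a message with the item's name.
; It then asks the Inventory to remove one unit at its stored Index and destroys itself if that call returns true.
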(event Custom|EventOnUsed
  (bind _iteminfo (Variables|Default|GetItemInfo))
  (bind (_name _description _icon _canbeused_) (Utilities|Struct|BreakS_Item_Info _iteminfo))
  (if _canbeused_
    (Development|PrintString (Utilities|String|Append "You Used " (Utilities|String|ToString(Text) _name)))
    (bind _success_ (Default|RemoveItematIndex (Variables|OnSpawn|GetInventory) (Variables|OnSpawn|GetIndex) 1))
    (if _success_
      (Actor|DestroyActor))))

(event EventBeginPlay)

(event Collision|EventActorBeginOverlap
  (params (OtherActor :type Actor%20Object%20Reference)))

(event EventTick
  (params (DeltaSeconds :type Float%20%28single-precision%29)))

(fn ConstructionScript)